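; BP_SpaceShip is the player-controlled spaceship pawn that moves on a plane and shoots lasers.
; Vertical and horizontal input axes offset it along world Z and Y with swept, frame-time-scaled movement.
; The Fire action spawns a BP_Laser at BulletSpawnPoint with itself as instigator, and hitting a BP_EnemyShip destroys the ship.
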(event Collision|EventHit
  (params (MyComp :type Primitive%20Component%20Object%20Reference) (Other :type Actor%20Object%20Reference) (OtherComp :type Primitive%20Component%20Object%20Reference) (bSelfMoved :type Boolean) (HitLocation :type Vector :default "0, 0, 0") (HitNormal :type Vector :default "0, 0, 0") (NormalImpulse :type Vector :default "0, 0, 0") (Hit :type Hit%20Result%20Structure%20%28by%20ref%29))
  (Utilities|FlowControl|Sequence
    (:then_0
      (Utilities|Casting|CastToBP_EnemyShip (.hitactor Hit))
      (Actor|DestroyActor))))

(event Input|ActionEvents|InputActionFire
  (params (Key :type Key%20Structure :default "AnyKey"))
  (:Pressed
    (Game|SpawnActorfromClass "/Game/Blueprints/Pawns/BP_Laser.BP_Laser_C" (Transformation|GetWorldTransform (Variables|Default|GetBulletSpawnPoint)) "AlwaysSpawn" 0 self)))

(event Input|AxisEvents|InputAxisHorizontalMove
  (params (AxisValue :type Float%20%28single-precision%29))
  ;[0 0 0] PlayerMovement
  (Transformation|AddActorWorldOffset (Math|Vector|MakeVector 0.0 (* AxisValue (* (Utilities|Time|GetWorldDeltaSeconds) (Variables|Default|GetMovementSpeed))) 0.0) true))

(event Input|AxisEvents|InputAxisVerticalMove
  (params (AxisValue :type Float%20%28single-precision%29))
  ;[0 0 0] PlayerMovement
  (Transformation|AddActorWorldOffset (Math|Vector|MakeVector 0.0 0.0 (* AxisValue (* (Utilities|Time|GetWorldDeltaSeconds) (Variables|Default|GetMovementSpeed)))) true))

(fn ConstructionScript)