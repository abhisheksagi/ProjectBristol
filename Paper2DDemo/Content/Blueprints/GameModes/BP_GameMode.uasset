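; Game mode for a ship game that sets a portrait screen resolution at startup and continuously spawns enemy ships.
; A looping timer fires the spawn event, which waits a random delay to stagger arrivals.
; Each BP_EnemyShip spawns at a random point in a box on the Y/Z plane with a random movement speed.
; The timer is cleared on EndPlay.
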(event Custom|SpawnEnemy
  (bind _returnvalue (Math|Random|RandomPointinBoundingBox (Math|Vector|MakeVector 0.0 0.0 0.0) (Math|Vector|MakeVector 0.0 1.3e+02 -2e+02)))
  ;[0.21 0 0] Random enemy spawning
  (Utilities|FlowControl|RetriggerableDelay (Math|Random|RandomFloatinRange 0.0 5.0))
  (Game|SpawnActorfromClass "/Game/Blueprints/Pawns/BP_EnemyShip.BP_EnemyShip_C" (Math|Transform|MakeTransform (Math|Vector|MakeVector 0.0 (.y _returnvalue) (.z _returnvalue)) "0, 0, 0" "1,1,1") "AlwaysSpawn" 0 (Math|Random|RandomFloatinRange 1e+01 4e+01) 0))

(event EventBeginPlay
  (Development|ExecuteConsoleCommand "r.setRes 640x960" (Game|GetPlayerController 0))
  (bind _returnvalue (Utilities|Time|SetTimerbyEvent (delegate Custom|SpawnEnemy) 6.0 true))
  (Variables|Default|SetSpawnTimerHandle _returnvalue))

(event EventEndPlay
  (params (EndPlayReason :type EEndPlayReason%20Enum))
  (Class|KismetSystemLibrary|ClearTimerHandle (Variables|Default|GetSpawnTimerHandle)))

(fn ConstructionScript)